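; BP_P38 is a player-controlled P-38 plane that pitches, rolls and fires rockets.
; BeginPlay registers both propellers with BPRotateActorComponent to spin on the X axis.
; Pitch and Roll inputs add frame-time-scaled local rotation, while Fire spawns a BP_Rocket at the Arrow's transform.
; Boost toggles Speed, but the forward AddMovementInput that reads it is disconnected, so this graph applies no forward movement.
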(event `self.ReceiveBeginPlay`
  (`/Game/Blueprints/BP_RotateActorComponent.AddRotateComponent` (`self.BP_RotateActorComponent`) (`self.LeftPropeller`))
  (`/Game/Blueprints/BP_RotateActorComponent.AddRotateComponent` (`self.BP_RotateActorComponent`) (`self.RightPropeller`))
  (set `/Game/Blueprints/BP_RotateActorComponent.RotateAxis` (struct :`Roll` 1.0) (`self.BP_RotateActorComponent`)))

(event `InputAxis|Pitch`
  (params (AxisValue :type "Float (single-precision)"))
  (`self.K2_AddActorLocalRotation` (`KismetMathLibrary.MakeRotator` 0.0 (* AxisValue (`self.RotationSpeed`) (`GameplayStatics.GetWorldDeltaSeconds`)))))

(event `InputAction|Boost`
  (params (Key :type "Key Structure"))
  (:`Pressed`
    (set `self.Speed` 1.0))
  (:`Released`
    (set `self.Speed` 0.5)))

(event `self.ReceiveTick`
  (params (DeltaSeconds :type "Float (single-precision)")))

(event `InputAction|Fire`
  (params (Key :type "Key Structure"))
  (:`Pressed`
    (`|SpawnActorFromClass` "/Game/Blueprints/BP_Rocket.BP_Rocket_C" (`SceneComponent.K2_GetComponentToWorld` (`self.Arrow`)) "Undefined" "MultiplyWithRoot" null null)))

(event `InputAxis|Roll`
  (params (AxisValue :type "Float (single-precision)"))
  (`self.K2_AddActorLocalRotation` (`KismetMathLibrary.MakeRotator` (* AxisValue (`self.RotationSpeed`) (`GameplayStatics.GetWorldDeltaSeconds`)))))

(fn `UserConstructionScript`)